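; PathSelectorManager is an actor that manages a ring of PathSelector child actors for choosing between path nodes.
; Its construction script resizes the ring to NumberOfSelectors, spaces selectors evenly by yaw, and assigns each an index and manager reference.
; SelectorHit uses nested loops over Nodes to call SetSelectedPath with the selected node and later nodes as previous.
; Selector on/off and delimiter visibility logic is disconnected.
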(event Custom|SelectorHit
  (params (SelectedIndex :type Integer))
  (bind _nodes (Variables|Default|GetNodes))
  ;[1 1 1] Set new selected path
  (for (_array_element _array_index) _nodes
    (for _index (range (+ _array_index 1) (- (Utilities|Array|Length _nodes) 1))
      (Class|PathNode|SetSelectedPath _array_element (Utilities|Array|Get(acopy) _nodes SelectedIndex) (Utilities|Array|Get(acopy) _nodes _index)))))

(event EventBeginPlay)

(event EventActorBeginOverlap
  (params (OtherActor :type Actor%20Object%20Reference)))

(event EventTick
  (params (DeltaSeconds :type Float%20%28single-precision%29)))

(fn ConstructionScript
  (bind _selectors (Variables|Default|GetSelectors))
  (bind _numberofselectors (Variables|Default|GetNumberOfSelectors))
  (bind _selectors_2 (Variables|Default|GetSelectors))
  (bind _numberofselectors_2 (Variables|Default|GetNumberOfSelectors))
  (bind _selectorselectedindices (Variables|Default|GetSelectorSelectedIndices))
  (bind _returnvalue (Utilities|Array|Length _selectors_2))
  ;[1 1 1] Determine size change
  (if (< _returnvalue _numberofselectors_2)
    ;[1 1 1] Add New Selectors
    (for _index (range (Utilities|Array|Length (Variables|Default|GetSelectors)) (- (Variables|Default|GetNumberOfSelectors) 1))
      (bind _returnvalue_2 (AddComponent|AddChildActorComponent false))
      (Utilities|Array|Add (Variables|Default|GetSelectors) _returnvalue_2))
    ;[1 1 1] Rotate all children
    (for _index_2 (range 0 (- _numberofselectors 1)) :!label _label
      (Transformation|SetRelativeRotation (Utilities|Array|Get(acopy) (Variables|Default|GetSelectors) _index_2) (Math|Rotator|MakeRotator 0.0 0.0 (* (/ 3.6e+02 (Math|Conversions|ToFloat(Integer) _numberofselectors)) (Math|Conversions|ToFloat(Integer) _index_2))) false false)
      ;[1 1 1] Trim indices array
      (for _index_3 (range (Variables|Default|GetNumberOfSelectors) (- (Utilities|Array|Length _selectorselectedindices) 1))
        (Utilities|Array|RemoveIndex _selectorselectedindices _index_3))
      ;[1 1 1] Set indices of selectors to those in array
      (for _index_4 (range 0 (- (Utilities|Array|Length (Variables|Default|GetSelectorSelectedIndices)) 1))
        (bind _aspath_selector (Utilities|Casting|CastToPathSelector (Variables|/Script/Engine.ChildActorComponent|GetChildActor (Utilities|Array|Get(acopy) (Variables|Default|GetSelectors) _index_4)))
          (:then
            (Variables|/Game/Blueprints/PathSelector.PathSelector_C|SetIndex _aspath_selector (Utilities|Array|Get(acopy) (Variables|Default|GetSelectorSelectedIndices) _index_4))
            (Variables|/Game/Blueprints/PathSelector.PathSelector_C|SetManager _aspath_selector self))
          (:CastFailed
            (Development|PrintString "Could not cast child actor to path selector!")))))
    (elif (> _returnvalue _numberofselectors_2)
      ;[1 1 1] Remove Old Selectors
      (for _index_5 (range (- (Variables|Default|GetNumberOfSelectors) 2) (- (Utilities|Array|Length _selectors) 1))
        (Components|DestroyComponent (Utilities|Array|Get(acopy) _selectors _index_5))
        (Utilities|Array|RemoveIndex _selectors _index_5))
      (goto _label))))
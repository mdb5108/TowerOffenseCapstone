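; AlliesManager tracks the player's Viking minions and decides when the game is won or lost.
; Minions are added to and removed from a list that keeps the live count, and removing the last one opens LoseLevel.
; IncrementWin tallies successful minions, and Tick prints a win message whenever that tally equals the live count, with no level change.
; BeginPlay also gives the game viewport focus and game-only input.
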(event EventBeginPlay
  (Class|WidgetBlueprintLibrary|SetFocustoGameViewport)
  (Input|SetInputModeGameOnly (Game|GetPlayerController 0)))

(event EventTick
  (params (DeltaSeconds :type Float%20%28single-precision%29))
  (if (== (Variables|Default|Getnumber_of_minions) (Variables|Default|GetWonMinions))
    (Development|PrintString "WIN!!" true true "(R=0.510000,G=0.145413,B=0.015300,A=1.000000)")))

(fn ConstructionScript)

(fn AddMinionstoList
  (params (InputViking :type Viking%20Minion%20Blueprint%20Object%20Reference))
  (bind _returnvalue (Utilities|Array|Add (Variables|Default|Getminions_list) InputViking))
  (Variables|Default|Setnumber_of_minions (Utilities|Array|Length (Variables|Default|Getminions_list))))

(fn DestroyMinionsfromList
  (params (DeleteMinion :type Viking%20Minion%20Object%20Reference))
  (bind _minions_list (Variables|Default|Getminions_list))
  ;[1 1 1] DeleteMinion and Set game state
  (bind (_array_element _array_index) (Utilities|Array|ForEachLoopwithBreak _minions_list :!label _label)
    (:LoopBody
      (if (== DeleteMinion _array_element)
        (Utilities|Array|RemoveIndex _minions_list _array_index)
        (goto _label Break)))
    (:Completed
      (bind _output_get (Variables|Default|Setnumber_of_minions (Utilities|Array|Length (Variables|Default|Getminions_list))))
      (if (== _output_get 0)
        (Game|OpenLevel(byName) "LoseLevel" (== _output_get 0))))))

(fn IncrementWin
  (Variables|Default|SetWonMinions (+ (Variables|Default|GetWonMinions) 1)))
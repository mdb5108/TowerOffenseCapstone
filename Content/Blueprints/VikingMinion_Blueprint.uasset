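; Viking minion ally character that registers itself with the AlliesManager on BeginPlay and gets a body tint and random name label in construction.
; Overlapping a FlamingBall-tagged actor removes it from the manager's list and destroys it after a short delay.
; A fast hit from the Player teleports it upward and launches it with amplified player velocity.
; SetDead increments the manager's WonMinions count rather than destroying the minion.
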(event EventActorBeginOverlap
  (params (OtherActor :type Actor%20Object%20Reference))
  (if (Actor|ActorHasTag OtherActor "FlamingBall")
    (Utilities|FlowControl|Delay 1.0)
    ;[1 1 1] Delete Minion from Manager then Destroy It
    (bind _outactors (Actor|GetAllActorsOfClass "/Game/Blueprints/AlliesManager.AlliesManager_C"))
    (Default|DestroyMinionsfromList _outactors self)
    (Actor|DestroyActor)))

(event EventTick
  (params (DeltaSeconds :type Float%20%28single-precision%29)))

(event EventBeginPlay
  ;[1 1 1] Add self to Allies Manager
  (bind _outactors (Actor|GetAllActorsOfClass "/Game/Blueprints/AlliesManager.AlliesManager_C"))
  (Default|AddMinionstoList _outactors self))

(event EventSetDead
  ;[1 1 1] Increment Number of Won minions
  (bind _outactors (Actor|GetAllActorsOfClass "/Game/Blueprints/AlliesManager.AlliesManager_C"))
  (for _array_element _outactors
    (Variables|/Game/Blueprints/AlliesManager.AlliesManager_C|SetWonMinions _array_element (+ (Variables|/Game/Blueprints/AlliesManager.AlliesManager_C|GetWonMinions _array_element) 1))))

(event Collision|EventHit
  (params (MyComp :type Primitive%20Component%20Object%20Reference) (Other :type Actor%20Object%20Reference) (OtherComp :type Primitive%20Component%20Object%20Reference) (bSelfMoved :type Boolean) (HitLocation :type Vector :default "0, 0, 0") (HitNormal :type Vector :default "0, 0, 0") (NormalImpulse :type Vector :default "0, 0, 0") (Hit :type Hit%20Result%20Structure%20%28by%20ref%29))
  (bind _returnvalue (Transformation|GetVelocity Other))
  (if (Actor|ActorHasTag Other "Player")
    (if (> (Math|Vector|VectorLength _returnvalue) 2e+02)
      (Collision|SetActorEnableCollision true)
      (Transformation|SetActorLocation (+ (Transformation|GetActorLocation) "0.000000,0.000000,100.000000") false true)
      (Variables|/Script/Engine.MovementComponent|SetVelocity (Pawn|GetMovementComponent (Pawn|GetControlledPawn (Pawn|GetController))) (+ (* _returnvalue 2) "0.000000,0.000000,120.000000"))
      (Utilities|FlowControl|Delay 0.0)
      (Collision|SetActorEnableCollision true)
      (Utilities|FlowControl|Delay 0.5)
      (Collision|SetActorEnableCollision true))))

(fn ConstructionScript
  (bind _returnvalue (Rendering|Material|CreateDynamicMaterialInstance (Variables|Character|GetMesh) 0 (Rendering|Material|GetMaterial (Variables|Character|GetMesh) 0) :!class /Script/Engine.PrimitiveComponent))
  (Rendering|Material|SetVectorParameterValue _returnvalue "BodyColor" (Math|Conversions|ToLinearColor(Vector) (Math|Vector|MakeVector 0.9 0.5 0.6)) :!class /Script/Engine.MaterialInstanceDynamic)
  (bind _returnvalue_2 (Class|VikingMinion|GetRandomName))
  (Rendering|Components|TextRender|SetText (Variables|Default|GetTextRender) (Utilities|Text|ToText(Name) _returnvalue_2)))
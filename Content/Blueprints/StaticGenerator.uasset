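; Static generator actor powering AffectedTowers, guarded by FatGuy child actors counted at BeginPlay.
; It records each FatGuy leaving the InBasket volume and disables the towers' shooting once all have left.
; While any remain, a VikingMinion entering AggroLimit triggers a one-time explosion: sphere-traced minion kills, radial impulse and particles, then self-destruction.
; A VikingMinion hit instead starts a delayed stepwise shrink that ends in destruction.
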(event OnComponentEndOverlap(InBasket)
  (params (OtherActor :type Actor%20Object%20Reference) (OtherComp :type Primitive%20Component%20Object%20Reference) (OtherBodyIndex :type Integer))
  (bind _returnvalue (Utilities|GetDisplayName OtherActor))
  ;[1 1 1] Test if Fatty has left
  (Utilities|Casting|CastToFatGuy OtherActor)
  (if (not (Utilities|Array|ContainsItem (Variables|Default|GetguySet) _returnvalue))
    (bind _returnvalue_2 (Utilities|Array|Add (Variables|Default|GetguySet) _returnvalue))
    (if (== _returnvalue_2 (- (Variables|Default|GetGuysCount) 1))
      (for _array_element (Variables|Default|GetaffectedTowers)
        (Default|DisableShooting _array_element)))))

(event OnComponentBeginOverlap(AggroLimit)
  (params (OtherActor :type Actor%20Object%20Reference) (OtherComp :type Primitive%20Component%20Object%20Reference) (OtherBodyIndex :type Integer) (bFromSweep :type Boolean) (SweepResult :type Hit%20Result%20Structure%20%28by%20ref%29))
  ;[1 1 1] Handle Explosions
  (if (< (Utilities|Array|Length (Variables|Default|GetguySet)) (Variables|Default|GetGuysCount))
    (if (Actor|ActorHasTag OtherActor "VikingMinion")
      (Utilities|FlowControl|DoOnce false
        (:Completed
          (CallFunction|Explode))))))

(event OnSystemFinished(ParticleSystem)
  (params (PSystem :type Particle%20System%20Component%20Object%20Reference))
  ;[1 1 1] Handle Explosions
  (Actor|DestroyActor))

(event EventBeginPlay
  ;[1 1 1] Get count of fatties
  (for _array_element (Components|GetChildrenComponents (Variables|Default|GetDefaultSceneRoot) false)
    (bind _aschild_actor_component (Utilities|Casting|CastToChildActorComponent _array_element))
    (if (== (Variables|/Script/Engine.ChildActorComponent|GetChildActorClass _aschild_actor_component) "/Game/Blueprints/FatGuy.FatGuy_C")
      (Math|Integer|IncrementInt (Variables|Default|GetGuysCount)))))

(event EventActorBeginOverlap
  (params (OtherActor :type Actor%20Object%20Reference)))

(event EventTick
  (params (DeltaSeconds :type Float%20%28single-precision%29)))

(event Collision|EventHit
  (params (MyComp :type Primitive%20Component%20Object%20Reference) (Other :type Actor%20Object%20Reference) (OtherComp :type Primitive%20Component%20Object%20Reference) (bSelfMoved :type Boolean) (HitLocation :type Vector :default "0, 0, 0") (HitNormal :type Vector :default "0, 0, 0") (NormalImpulse :type Vector :default "0, 0, 0") (Hit :type Hit%20Result%20Structure%20%28by%20ref%29))
  ;[1 1 1] Handle minion diffuse
  (if (Actor|ActorHasTag Other "VikingMinion")
    (Utilities|FlowControl|Delay 1.0)
    (Utilities|FlowControl|Sequence
      (:then_0
        (Transformation|SetActorRelativeScale3D (* (Class|Actor|GetActorRelativeScale3D self) 0.9) :!label _label)
        (Utilities|FlowControl|Delay 0.2)
        (if (Variables|Default|GetstopScaleDelay)
          (Variables|Default|SetstopScaleDelay false)
          (Actor|DestroyActor)
          (else
            (goto _label))))
      (:then_1
        (Utilities|FlowControl|Delay 3.0)
        (Variables|Default|SetstopScaleDelay true)))))

(fn ConstructionScript)

(fn Explode
  (bind _self self)
  (bind _defaultsceneroot (Variables|Default|GetDefaultSceneRoot _self))
  (bind _returnvalue (Transformation|GetWorldLocation _defaultsceneroot))
  (Utilities|FlowControl|Sequence
    (:then_0
      (bind _outhits (Class|KismetSystemLibrary|SphereTraceMultiNEW _returnvalue (+ _returnvalue "1.000000, 0, 0") (Variables|/Script/Engine.RadialForceComponent|GetRadius (Variables|Default|GetRadialForce)) "TraceTypeQuery3" false 0 "Persistent" true))
      (for _array_element _outhits
        (bind _asviking_minion_blueprint (Utilities|Casting|CastToVikingMinion_Blueprint (.HitActor (Collision|BreakHitResult _array_element))))
        (Default|Die _asviking_minion_blueprint)))
    (:then_1
      (Class|RadialForceComponent|FireImpulse (Variables|Default|GetRadialForce)))
    (:then_2
      (Components|Activation|SetActive (Variables|Default|GetParticleSystem) true false))))
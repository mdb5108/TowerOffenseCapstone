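; FatGuy is a physics-driven actor that gets released from its constraint and pushed when struck by an actor tagged FlamingBall.
; Capsule hits, AggroLimit component hits and actor overlaps all feed TryCollision, which ignores StaticGenerator, Landscape and other FatGuys.
; A qualifying collision sets the capsule's constraint mode to None and applies an impulse from the negated hit normal or overlap direction.
; Tick clamps the capsule's linear velocity to MaxVelocity.
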(event OnComponentHit(AggroLimit)
  (params (OtherActor :type Actor%20Object%20Reference) (OtherComp :type Primitive%20Component%20Object%20Reference) (NormalImpulse :type Vector) (Hit :type Hit%20Result%20Structure%20%28by%20ref%29))
  (CallFunction|TryCollision OtherActor (Math|Vector|NegateVector NormalImpulse)))

(event Custom|TryCollision
  (params (other :type Actor%20Object%20Reference) (impulse :type Vector))
  (Utilities|Casting|CastToStaticGenerator other
    (:CastFailed
      (Utilities|Casting|CastToLandscape other
        (:CastFailed
          (Utilities|Casting|CastToFatGuy other
            (:CastFailed
              (if (Actor|ActorHasTag other "FlamingBall")
                (Class|PrimitiveComponent|SetConstraintMode (Variables|Default|GetCapsule) "None")
                (Physics|AddImpulse (Variables|Default|GetCapsule) (* impulse 1.0) "None" false)))))))))

(event EventTick
  (params (DeltaSeconds :type Float%20%28single-precision%29))
  (bind _returnvalue (Transformation|GetVelocity))
  (bind _maxvelocity (Variables|Default|GetMaxVelocity))
  (if (< (Math|Float|Square _maxvelocity) (Math|Vector|VectorLengthSquared _returnvalue))
    (Physics|SetPhysicsLinearVelocity (Variables|Default|GetCapsule) (* (Math|Vector|Normalize _returnvalue) _maxvelocity) false "None")
    (else
      (Physics|SetPhysicsLinearVelocity (Variables|Default|GetCapsule) _returnvalue false "None"))))

(event Collision|EventHit
  (params (MyComp :type Primitive%20Component%20Object%20Reference) (Other :type Actor%20Object%20Reference) (OtherComp :type Primitive%20Component%20Object%20Reference) (bSelfMoved :type Boolean) (HitLocation :type Vector :default "0, 0, 0") (HitNormal :type Vector) (NormalImpulse :type Vector) (Hit :type Hit%20Result%20Structure%20%28by%20ref%29))
  (CallFunction|TryCollision Other (Math|Vector|NegateVector NormalImpulse)))

(event Collision|EventActorBeginOverlap
  (params (OtherActor :type Actor%20Object%20Reference))
  (CallFunction|TryCollision OtherActor (Math|Vector|Normalize (- (Transformation|GetActorLocation) (Transformation|GetActorLocation OtherActor)))))

(fn ConstructionScript)
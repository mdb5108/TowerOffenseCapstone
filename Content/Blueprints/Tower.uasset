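; Tower actor that periodically spawns an enlarged FlamingBall high above itself while Shooting is true.
; Tick runs a Delay as a repeating fire timer, rechecks Shooting, then spawns the ball rotated relative to the tower's own rotation.
; A DisableShooting event clears the flag to stop firing.
; Trigger overlaps track the player pawn in IsOverlapping, but firing ignores it, and player-aiming nodes are left unconnected.
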(event OnComponentBeginOverlap(Trigger)
  (params (OtherActor :type Actor%20Object%20Reference) (OtherComp :type Primitive%20Component%20Object%20Reference) (OtherBodyIndex :type Integer) (bFromSweep :type Boolean) (SweepResult :type Hit%20Result%20Structure%20%28by%20ref%29))
  (if (== OtherActor (Game|Player|GetPlayerPawn 0))
    (Variables|Default|SetisOverlapping true)))

(event OnComponentEndOverlap(Trigger)
  (params (OtherActor :type Actor%20Object%20Reference) (OtherComp :type Primitive%20Component%20Object%20Reference) (OtherBodyIndex :type Integer))
  (if (== (Game|Player|GetPlayerPawn 0) OtherActor)
    (Variables|Default|SetisOverlapping false)))

(event Custom|DisableShooting
  (Variables|Default|Setshooting false))

(event EventTick
  (params (DeltaSeconds :type Float%20%28single-precision%29)))

(event EventTick
  (params (DeltaSeconds :type Float%20%28single-precision%29))
  (if (Variables|Default|Getshooting)
    (Utilities|FlowControl|Delay 5.0)
    (if (Variables|Default|Getshooting)
      (Game|SpawnActorfromClass "/Game/Blueprints/FlamingBall.FlamingBall_C" (Math|Transform|MakeTransform (+ (Transformation|GetActorLocation) "0, 0,2000.000000") (Math|Rotator|CombineRotators "30.000000,270.000000,0.000000" (Transformation|GetActorRotation)) "4.000000,4.000000,4.000000") "Undefined" 0 0))))

(fn ConstructionScript)
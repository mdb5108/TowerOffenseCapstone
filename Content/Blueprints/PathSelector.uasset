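; PathSelector is a trigger actor that reports to its Manager, passing its own Index, whenever another actor overlaps it.
; The construction script creates a dynamic material on the Delimiter component and sets its BodyColor to the start color.
; TurnOn and TurnOff events switch that color between the end and start values.
; The overlap does not filter the other actor and also prints a debug string.
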(event Custom|TurnOff
  (Rendering|Material|SetVectorParameterValue (Variables|Default|GetMaterialInstance) "BodyColor" (Variables|Default|GetColorStart) :!class /Script/Engine.MaterialInstanceDynamic))

(event Custom|TurnOn
  (Rendering|Material|SetVectorParameterValue (Variables|Default|GetMaterialInstance) "BodyColor" (Variables|Default|GetColorEnd) :!class /Script/Engine.MaterialInstanceDynamic))

(event EventBeginPlay)

(event EventActorBeginOverlap
  (params (OtherActor :type Actor%20Object%20Reference))
  (Default|SelectorHit (Variables|Default|GetManager) (Variables|Default|GetIndex))
  (Development|PrintString "Hello"))

(event EventTick
  (params (DeltaSeconds :type Float%20%28single-precision%29)))

(fn ConstructionScript
  (bind _returnvalue (Rendering|Material|CreateDynamicMaterialInstance (Variables|Default|Getdelimiter) 0 (Rendering|Material|GetMaterial (Variables|Default|Getdelimiter) 0) :!class /Script/Engine.PrimitiveComponent))
  (bind _output_get (Variables|Default|SetMaterialInstance _returnvalue))
  (Rendering|Material|SetVectorParameterValue _output_get "BodyColor" (Variables|Default|GetColorStart) :!class /Script/Engine.MaterialInstanceDynamic))